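; BP_MyActor is a setup actor that creates a hands interface widget, spawns a triangle mesh actor and drives a noise texture generator.
; On BeginPlay it initializes itself, passes itself to WI_HandsInterface and BP_TriangleMesh, and generates a small noise texture.
; A looping timer then updates that texture every few seconds with random U and V values.
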(event Custom|CustomEvent
  (Class|NoiseGenerator|UpdateNoiseTexture (stale EventBeginPlay _returnvalue_2) (Math|Random|RandomFloat) (Math|Random|RandomFloat)))

(event EventBeginPlay
  (Class|MyActor|Initialize)
  (bind _returnvalue (UserInterface|CreateWidget "/Game/WI_HandsInterface.WI_HandsInterface_C" 0 self))
  (UserInterface|Viewport|AddtoViewport _returnvalue 0)
  (Game|SpawnActorfromClass "/Game/BP_TriangleMesh.BP_TriangleMesh_C" (Math|Transform|MakeTransform "0, 0, 0" "0, 0, 0" "1.000000,1.000000,1.000000") "Undefined" "MultiplyWithRoot" 0 self 0)
  (bind _returnvalue_2 (Class|MyActor|GetNoiseGenerator))
  (Class|NoiseGenerator|GenerateNoiseTexture _returnvalue_2 50 50 1.0 0.5 0.5)
  (Utilities|Time|SetTimerbyEvent (delegate Custom|CustomEvent) 2.0 true))

(event Collision|EventActorBeginOverlap
  (params (OtherActor :type Actor%20Object%20Reference)))

(event EventTick
  (params (DeltaSeconds :type Float%20%28single-precision%29)))

(fn ConstructionScript)